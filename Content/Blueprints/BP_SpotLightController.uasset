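; BP_SpotLightController is a road light that periodically flickers its spotlight and glowing mesh.
; On BeginPlay it starts a looping timer and swaps the LightRoad mesh material for a dynamic instance.
; Each timer tick runs a delay-chained blink sequence that toggles spotlight intensity alongside the material's emissive scalar parameter, with a brief dimmer step before returning to full brightness.
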(event `self.ReceiveBeginPlay`
  (`|ExecutionSequence`
    (:`then_0`
      (`KismetSystemLibrary.K2_SetTimerDelegate` (delegate `StartBlinking`) 8.0 true))
    (:`then_1`
      (bind _returnvalue (`KismetMaterialLibrary.CreateDynamicMaterialInstance` (`PrimitiveComponent.GetMaterial` (`self.Light_Road`) 0)))
      (`PrimitiveComponent.SetMaterial` (`self.Light_Road`) 0 _returnvalue)
      (set `self.EmissiveMat` _returnvalue))))

(event `StartBlinking`
  (`self.LR-EmissiveOff`)
  (`LightComponent.SetIntensity` (`self.SpotLightComponent`) 0.0)
  (`KismetSystemLibrary.Delay` 0.3)
  (`self.LR-EmissiveOn`)
  (`LightComponent.SetIntensity` (`self.SpotLightComponent`) 100000.0)
  (`KismetSystemLibrary.Delay` 0.1)
  (`self.LR-EmissiveOff`)
  (`LightComponent.SetIntensity` (`self.SpotLightComponent`) 0.0)
  (`KismetSystemLibrary.Delay` 0.1)
  (`self.LR-EmissiveOn`)
  (`LightComponent.SetIntensity` (`self.SpotLightComponent`) 20000.0)
  (`KismetSystemLibrary.Delay` 0.2)
  (`LightComponent.SetIntensity` (`self.SpotLightComponent`) 100000.0))

(event `LR-EmissiveOff`
  (`MaterialInstanceDynamic.SetScalarParameterValue` (`self.EmissiveMat`) "EmissiveParam" 0.0))

(event `LR-EmissiveOn`
  (`MaterialInstanceDynamic.SetScalarParameterValue` (`self.EmissiveMat`) "EmissiveParam" 5.0))

(fn `UserConstructionScript`)